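; Human character Blueprint that manages health and oxygen survival, shown through a HumanUI widget component and skull and heal effects.
; Tick raises or drains oxygen depending on the oxygenated state, healing at full oxygen and applying suffocation damage when empty.
; DealDamage scales by frame delta, clamps health and reports death, which triggers OnDeathEvent.
; A separate OnDeath_Event handler loads the MainMenu level.
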(event `self.ReceiveTick`
  (params (DeltaSeconds :type "Float (single-precision)"))
  (bind _skulls (`self.skulls`))
  (bind _heals (`self.heals`))
  (bind _oxygen (`self.Oxygen`))
  (`|ExecutionSequence`
    (:`then_0`
      (bind _ashuman_ui (cast `/Game/Blueprint/Widgets/HumanUI` (`WidgetComponent.GetUserWidgetObject` (`self.Health & Oxygen`)))
        (:`then`
          (`/Game/Blueprint/Widgets/HumanUI.ChangeHPTo` _ashuman_ui (/ (`self.Health`) 100.0))
          (`/Game/Blueprint/Widgets/HumanUI.ChangeOxygenTo` _ashuman_ui (/ (`self.Oxygen`) 100.0)))
        (:`CastFailed`
          (`KismetSystemLibrary.PrintString` "BAD WIDGET IN HUMAN")))
      (if (`self.InOxygenatedState`)
        (bind _output_get (set `self.Oxygen` (+ (`self.Oxygen`) (* DeltaSeconds (`self.OxygenGainPerSecond`)))))
        (if (> _output_get 100.0)
          (set `self.Oxygen` 100.0)
          (`self.DealDamage` (* (`self.HealthGainPerSecond`) -1.0)))
        (`SceneComponent.SetVisibility` (`self.skulls`) false false)
        (else
          (set `self.Oxygen` (- _oxygen (* DeltaSeconds (`self.OxygenLossPerSecond`))))
          (if (<= _oxygen 0.1)
            (if (< (`self.Oxygen`) 0.0)
              (set `self.Oxygen` 0.0)
              (`ActorComponent.Activate` _skulls false)
              (`SceneComponent.SetVisibility` _skulls true false))
            (bind _isdead (`self.DealDamage` (`self.SuffocationPerSecond`)))
            (if _isdead
              (`self.OnDeath_Event`))))))
    (:`then_1`
      (if (< (`self.Oxygen`) 99.5)
        (`SceneComponent.SetVisibility` (`self.heals`) false false)
        (elif (< (`self.Health`) 100.0)
          (`ActorComponent.Activate` _heals false)
          (`SceneComponent.SetVisibility` _heals true false)
          (else
            (`SceneComponent.SetVisibility` (`self.heals`) false false)))))))

(event `OnDeath_Event`
  (`GameplayStatics.OpenLevel` "MainMenu"))

(fn `DealDamage`
  (params (DamageAmount :type "Float (double-precision)"))
  (returns (IsDead :type Boolean))
  (bind _health (`self.Health`))
  (bind _output_get (set `self.Health` (- _health (* DamageAmount (`GameplayStatics.GetWorldDeltaSeconds`)))))
  (if (> _output_get 100.0)
    (set `self.Health` 100.0))
  (if (< _output_get 0.0)
    (set `self.Health` 0.0))
  (return (<= _health 0.1)))

(fn `RemoveOxygen`
  (params (OxygenToRemove :type "Float (double-precision)"))
  (returns (OutOfOxygen :type Boolean))
  (bind _oxygen (`self.Oxygen`))
  (set `self.Oxygen` (- _oxygen OxygenToRemove))
  (return (<= _oxygen 0.0)))

(fn `SetOxygenatedState`
  (params (NewState :type Boolean))
  (`self.SetOxygenatedState` NewState))

(fn `UserConstructionScript`)