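; Game mode for a local multiplayer droid game that spawns Welder, Electrician, Support and Janitor droids and shows a droid select widget.
; Extra players from the game instance's player count are created to possess the first uncontrolled droid.
; Tick feeds the droid references into the widget's cover state.
; A looping delay-based event randomly starts, repeats and clears game events, whose effect so far only prints a random tile's name.
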(event `self.ReceiveBeginPlay`
  (bind (_asgame_instance_bp _bsuccess) (cast `/Game/Blueprint/GameInstanceBP` (`GameplayStatics.GetGameInstance`) :!pure true))
  (`self.BeginGame`)
  (if _bsuccess
    (for _ (range (+ (- (`/Game/Blueprint/GameInstanceBP.NumberOfPlayers` _asgame_instance_bp) 2) 1))
      (`self.DropPlayerIn` (`self.GetUnpossessedPlayer`)))))

(event `self.ReceiveTick`
  (params (DeltaSeconds :type "Float (single-precision)"))
  (`/Game/Blueprint/Widgets/DroidSelect.SetCoverState` (`self.DroidSelectWidget`) (`self.DElectrician`) (`self.DJanitor`) (`self.DWelder`) (`self.DMedic`)))

(event `Begin Game Event Loop`
  (if (`|EnumInequality` (`self.currentGameEvent`)) :!label _label
    (`self.DoGameEvent` (`self.currentGameEvent`))
    (if (`KismetMathLibrary.RandomBoolWithWeight` 0.1)
      (set `self.currentGameEvent` "None") ; Reset Event
      (`KismetSystemLibrary.Delay` 45.0)
      (goto _label)
      (else
        (`KismetSystemLibrary.Delay` (`KismetMathLibrary.RandomFloatInRange` 1.0 30.0))
        (goto _label)))
    (else
      (`KismetSystemLibrary.Delay` 1.0)
      (if (`KismetMathLibrary.RandomBoolWithWeight` 0.1)
        (bind _returnvalue (`self.GetRandomGameEvent`))
        (bind _output_get (set `self.currentGameEvent` _returnvalue))
        (`KismetSystemLibrary.PrintString` (`|GetEnumeratorNameAsString` _output_get) true true (struct :`G` 0.66 :`B` 1.0 :`A` 1.0) 9999.0)
        (goto _label)
        (else
          (goto _label))))))

(event `self.DoGameEvent`
  (params (current :type "EGameEvent Enum" :default "None"))
  (bind _returnvalue (`self.GetRandomTile`)) ; F*ck up a random tile
  (`KismetSystemLibrary.PrintString` (`KismetSystemLibrary.GetObjectName` _returnvalue)))

(fn `BeginGame`
  (`|ExecutionSequence`
    (:`then_0`
      (set `self.InGame` true)
      (bind _returnvalue (`|SpawnActorFromClass` "/Game/Blueprint/Droids/WelderDroid.WelderDroid_C" (`KismetMathLibrary.MakeTransform` (-200.0 0.0 100.0)) "AdjustIfPossibleButAlwaysSpawn" "OverrideRootScale" null null))
      (set `self.DWelder` _returnvalue)
      (bind _returnvalue_2 (`|SpawnActorFromClass` "/Game/Blueprint/Droids/ElectricianDroid.ElectricianDroid_C" (`KismetMathLibrary.MakeTransform` (-100.0 0.0 100.0)) "AdjustIfPossibleButAlwaysSpawn" "OverrideRootScale" null null))
      (set `self.DElectrician` _returnvalue_2)
      (bind _returnvalue_3 (`|SpawnActorFromClass` "/Game/Blueprint/Droids/SupportDroid.SupportDroid_C" (`KismetMathLibrary.MakeTransform` (0.0 0.0 100.0)) "AdjustIfPossibleButAlwaysSpawn" "OverrideRootScale" null null))
      (set `self.DMedic` _returnvalue_3)
      (bind _returnvalue_4 (`|SpawnActorFromClass` "/Game/Blueprint/Droids/JanitorDroid.JanitorDroid_C" (`KismetMathLibrary.MakeTransform` (100.0 0.0 100.0)) "AdjustIfPossibleButAlwaysSpawn" "OverrideRootScale" null null))
      (set `self.DJanitor` _returnvalue_4))
    (:`then_1`
      (bind _returnvalue_5 (`|CreateWidget` "/Game/Blueprint/Widgets/DroidSelect.DroidSelect_C"))
      (bind _output_get (set `self.DroidSelectWidget` _returnvalue_5))
      (`UserWidget.AddToViewport` _output_get 0))
    (:`then_2`
      (`self.Begin Game Event Loop`))))

(fn `DropPlayerIn`
  (params (DroidToPossess :type "BaseDroid Object Reference"))
  (bind _returnvalue (`GameplayStatics.CreatePlayer` -1))
  (`Controller.Possess` _returnvalue DroidToPossess))

(fn `DropPlayerOut`
  (params (PlayerToRemove :type "DroidPlayerController Object Reference"))
  (`GameplayStatics.RemovePlayer` PlayerToRemove))

(fn `GetUnpossessedPlayer`
  (returns (`Available Droid` :type "BaseDroid Object Reference"))
  (bind _dwelder (`self.DWelder`))
  (bind _delectrician (`self.DElectrician`))
  (bind _dmedic (`self.DMedic`))
  (bind _djanitor (`self.DJanitor`))
  (if (not (`Pawn.IsControlled` _dwelder))
    (return _dwelder)
    (elif (not (`Pawn.IsControlled` _delectrician))
      (return _delectrician)
      (elif (not (`Pawn.IsControlled` _dmedic))
        (return _dmedic)
        (elif (not (`Pawn.IsControlled` _djanitor))
          (return _djanitor)
          (else
            (return null)))))))

(fn `UserConstructionScript`)