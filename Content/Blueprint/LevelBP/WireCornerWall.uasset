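; Wire corner wall piece, a repairable level object that shows spark effects while damaged.
; Tick polls NeedRepair and the repair queue, activating and showing four spark components when repair is needed and the queue length is not one.
; Otherwise it only hides the sparks, without deactivating them.
; OnRepair simply forwards to the parent class, which supplies the repair behavior.
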(event `self.ReceiveTick`
  (params (DeltaSeconds :type "Float (single-precision)"))
  (bind _sparks (`self.Sparks`))
  (bind _sparks1 (`self.Sparks1`))
  (bind _sparks2 (`self.Sparks2`))
  (bind _sparks3 (`self.Sparks3`))
  (if (and (`self.NeedRepair`) (!= (`KismetArrayLibrary.Array_Length` (`self.m_RepairQueue`)) 1))
    (`ActorComponent.Activate` _sparks false)
    (`SceneComponent.SetVisibility` _sparks true false)
    (`ActorComponent.Activate` _sparks1 false)
    (`SceneComponent.SetVisibility` _sparks1 true false)
    (`ActorComponent.Activate` _sparks2 false)
    (`SceneComponent.SetVisibility` _sparks2 true false)
    (`ActorComponent.Activate` _sparks3 false)
    (`SceneComponent.SetVisibility` _sparks3 true false)
    (else
      (`SceneComponent.SetVisibility` _sparks false false)
      (`SceneComponent.SetVisibility` _sparks1 false false)
      (`SceneComponent.SetVisibility` _sparks2 false false)
      (`SceneComponent.SetVisibility` _sparks3 false false))))

(event `self.OnRepair`
  (params (old :type "ERepairType Enum" :default "FixWiring"))
  (`parent.OnRepair` old))

(fn `UserConstructionScript`)