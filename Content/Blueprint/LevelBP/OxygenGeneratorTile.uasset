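; OxygenGeneratorTile is a level Blueprint tile that shows particle effects while the oxygen generator needs repair.
; Every Tick it polls NeedRepair, which is not defined in this graph, and switches three particle system components to match.
; When repair is needed it activates them without reset and makes them visible; otherwise it only hides them, without deactivating.
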(event `self.ReceiveTick`
  (params (DeltaSeconds :type "Float (single-precision)"))
  (bind _particlesystem1 (`self.ParticleSystem1`))
  (bind _particlesystem2 (`self.ParticleSystem2`))
  (bind _particlesystem (`self.ParticleSystem`))
  (if (`self.NeedRepair`)
    (`ActorComponent.Activate` _particlesystem false)
    (`SceneComponent.SetVisibility` _particlesystem true false)
    (`ActorComponent.Activate` _particlesystem1 false)
    (`SceneComponent.SetVisibility` _particlesystem1 true false)
    (`ActorComponent.Activate` _particlesystem2 false)
    (`SceneComponent.SetVisibility` _particlesystem2 true false)
    (else
      (`SceneComponent.SetVisibility` (`self.ParticleSystem`) false false)
      (`SceneComponent.SetVisibility` (`self.ParticleSystem1`) false false)
      (`SceneComponent.SetVisibility` (`self.ParticleSystem2`) false false))))

(fn `UserConstructionScript`)