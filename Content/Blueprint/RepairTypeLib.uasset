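; Function library that creates the skill check widget for a given repair type.
; CreateWidgetFromRepairType maps the hold, mash and timed press types to their widget classes and returns the new widget owned by the passed player controller.
; The random type rolls an integer, converts it through GetSkillcheckTypeFromInt and recursively calls the create function with the concrete type.
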(fn `CreateWidgetFromRepairType`
  (params (`Skill Check` :type "ESkillCheckType Enum" :default "HoldButtonDown") (PController :type "PlayerController Object Reference"))
  (returns (SkillCheck :type "/Game/Blueprint/ISkillCheck Interface"))
  (locals (PlayerController :type "PlayerController Object Reference"))
  (bind ___worldcontext (`local.__WorldContext`))
  (set `local.PlayerController` PController)
  (switch `ESkillCheckType` `Skill Check`
    (:`HoldButtonDown`
      (bind _returnvalue (`|CreateWidget` "/Game/Blueprint/ButtonHold.ButtonHold_C" (`local.PlayerController`)))
      (return _returnvalue))
    (:`MashButton`
      (bind _returnvalue_2 (`|CreateWidget` "/Game/Blueprint/TheMonsterMash.TheMonsterMash_C" (`local.PlayerController`)))
      (return _returnvalue_2))
    (:`TimedPress`
      (bind _returnvalue_3 (`|CreateWidget` "/Game/Blueprint/TimedSkillCheck.TimedSkillCheck_C" (`local.PlayerController`)))
      (return _returnvalue_3))
    (:`RandomCheck`
      (bind _repair_type (`self.GetSkillcheckTypeFromInt` (`KismetMathLibrary.RandomIntegerInRange` 0 2) ___worldcontext))
      (bind _skillcheck (`self.CreateWidgetFromRepairType` _repair_type PController ___worldcontext))
      (return _skillcheck))))

(fn `GetSkillcheckTypeFromInt`
  (params (Int :type Integer))
  (returns (`repair type` :type "ESkillCheckType Enum"))
  (switch `int` Int
    (:`Default`
      (return "HoldButtonDown"))
    (:`0`
      (return "HoldButtonDown"))
    (:`1`
      (return "MashButton"))
    (:`2`
      (return "TimedPress"))))