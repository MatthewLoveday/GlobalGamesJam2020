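; DroidBP is a controllable droid that repairs tile layers through skillcheck minigames.
; Interacting with a tile caches it and creates the skillcheck widget matching its current repair type.
; Skillcheck button presses and releases are forwarded to that widget, which Tick polls for completion.
; A finished check removes the widget, then either repairs the tile's layer on success or cancels the interaction.
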(event `self.ReceiveBeginPlay`)

(event `self.OnSkillcheckDown`
  (bind _currentskillcheck (`self.CurrentSkillcheck`))
  (`/Engine/EditorBlueprintResources/StandardMacros.IsValid` _currentskillcheck
    (:`Is Valid`
      (message `/Game/Blueprint/ISkillCheck.ActionButtonDown` _currentskillcheck))))

(event `self.OnSkillcheckUp`
  (bind _currentskillcheck (`self.CurrentSkillcheck`))
  (`/Engine/EditorBlueprintResources/StandardMacros.IsValid` _currentskillcheck
    (:`Is Valid`
      (message `/Game/Blueprint/ISkillCheck.ActionButtonUp` _currentskillcheck))))

(event `self.InteractWithTile`
  (params (tile :type "TileBase Object Reference"))
  (`parent.InteractWithTile` tile)
  (bind _output_get (set `self.CachedTile` tile))
  (bind _returnvalue (`TileBase.GetCurrentRepairType` _output_get))
  (set `self.CurrentSkillcheck` (`/Game/Blueprint/RepairTypeLib.CreateWidgetFromRepairType` (`.skillcheckType` (break `RepairData` (`TileBase.SearchArrayForRepairType` _output_get _returnvalue))) (cast `PlayerController` (`self.GetController`) :!pure true))))

(event `self.ReceiveTick`
  (params (DeltaSeconds :type "Float (single-precision)"))
  (if (`KismetSystemLibrary.IsValid` (`self.CurrentSkillcheck`))
    (bind (_completed _success) (message `/Game/Blueprint/ISkillCheck.PollSkillCheck` (`self.CurrentSkillcheck`)))
    (if _completed
      (`Widget.RemoveFromParent` (`self.CurrentSkillcheck`))
      (if _success
        (`self.OnRepairComplete`)
        (else
          (`self.CancelInteraction`))))))

(event `self.OnRepairComplete`
  (`parent.OnRepairComplete`)
  (`TileBase.RepairLayer` (`self.CachedTile`))
  (set `self.CurrentSkillcheck` null)
  (set `self.CachedTile` null))

(fn `UserConstructionScript`)