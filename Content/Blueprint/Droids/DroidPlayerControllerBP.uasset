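; Player controller that lets a player switch between the electrician, welder, janitor and support droids.
; Input actions fetch each droid from DroidGameModeBP and possess it only if it is not already controlled.
; On possession it creates a NeedsCharacter hint widget if none exists.
; Each tick, that hint shows the droid required by the repair type of the tile in front of the controlled droid, and hides when none applies.
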(event `self.ReceivePossess`
  (params (PossessedPawn :type "Pawn Object Reference"))
  (`/Engine/EditorBlueprintResources/StandardMacros.IsValid` (`self.needsCharacter`)
    (:`Is Not Valid`
      (bind _returnvalue (`|CreateWidget` "/Game/Blueprint/Widgets/NeedsCharacterHint.NeedsCharacterHint_C" self))
      (bind _output_get (set `self.needsCharacter` _returnvalue))
      (`UserWidget.AddToPlayerScreen` _output_get 0))))

(event `self.ReceiveBeginPlay`)

(event `InputAction|SelectElectrician`
  (params (Key :type "Key Structure"))
  (:`Pressed`
    (bind _asdroid_game_mode_bp (cast `/Game/Blueprint/DroidGameModeBP` (`GameplayStatics.GetGameMode`)))
    (`self.PossessIfAvailable` (`/Game/Blueprint/DroidGameModeBP.DElectrician` _asdroid_game_mode_bp))))

(event `InputAction|SelectWelder`
  (params (Key :type "Key Structure"))
  (:`Pressed`
    (bind _asdroid_game_mode_bp (cast `/Game/Blueprint/DroidGameModeBP` (`GameplayStatics.GetGameMode`)))
    (`self.PossessIfAvailable` (`/Game/Blueprint/DroidGameModeBP.DWelder` _asdroid_game_mode_bp))))

(event `InputAction|SelectJanitor`
  (params (Key :type "Key Structure"))
  (:`Pressed`
    (bind _asdroid_game_mode_bp (cast `/Game/Blueprint/DroidGameModeBP` (`GameplayStatics.GetGameMode`)))
    (`self.PossessIfAvailable` (`/Game/Blueprint/DroidGameModeBP.DJanitor` _asdroid_game_mode_bp))))

(event `InputAction|SelectSupport`
  (params (Key :type "Key Structure"))
  (:`Pressed`
    (bind _asdroid_game_mode_bp (cast `/Game/Blueprint/DroidGameModeBP` (`GameplayStatics.GetGameMode`)))
    (`self.PossessIfAvailable` (`/Game/Blueprint/DroidGameModeBP.DMedic` _asdroid_game_mode_bp))))

(event `self.ReceiveTick`
  (params (DeltaSeconds :type "Float (single-precision)"))
  (bind _asbase_droid (cast `BaseDroid` (`self.K2_GetPawn`)))
  (bind _tileinfrontregardlessofvalidity (`BaseDroid.tileInFrontRegardlessOfValidity` _asbase_droid))
  (`/Engine/EditorBlueprintResources/StandardMacros.IsValid` _tileinfrontregardlessofvalidity
    (:`Is Valid`
      (bind _asdroid_game_mode_bp (cast `/Game/Blueprint/DroidGameModeBP` (`GameplayStatics.GetGameMode`)))
      (bind _returnvalue (`TileBase.GetCurrentRepairType` _tileinfrontregardlessofvalidity))
      (if (not (`|EnumEquality` _returnvalue))
        (bind _droid (`/Game/Blueprint/DroidGameModeBP.GetDroidFromRepairType` _asdroid_game_mode_bp _returnvalue))
        (`/Game/Blueprint/Widgets/NeedsCharacterHint.SetIconFromDroid` (`self.needsCharacter`) _droid)
        (`Widget.SetVisibility` (`self.needsCharacter`) "Visible")
        (else
          (`Widget.SetVisibility` (`self.needsCharacter`) "Hidden"))))
    (:`Is Not Valid`
      (`Widget.SetVisibility` (`self.needsCharacter`) "Hidden"))))

(fn `AddWidget`
  (params (Widget :type "UserWidget Class Reference"))
  (returns (CreatedWidget :type "UserWidget Object Reference"))
  (bind _returnvalue (`|CreateWidget` Widget self))
  (`UserWidget.AddToPlayerScreen` _returnvalue 0)
  (return _returnvalue))

(fn `PossessIfAvailable`
  (params (droid :type "BaseDroid Object Reference"))
  (if (not (`Pawn.IsControlled` droid))
    (`self.Possess` droid)
    (return)))

(fn `UserConstructionScript`)