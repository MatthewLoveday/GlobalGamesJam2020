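; Dispenser actor that keeps a fresh pickup available at its spawn point.
; BeginPlay spawns a PickupClass actor at the SpawnPos location and tracks it as CurrentSpawnedItem.
; Tick polls that item's IsBeingCarried flag and, once it is set, spawns and tracks a replacement at the same spot.
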(event `self.ReceiveBeginPlay`
  (bind _returnvalue (`|SpawnActorFromClass` (`self.PickupClass`) (`KismetMathLibrary.Conv_VectorToTransform` (`SceneComponent.K2_GetComponentLocation` (`self.spawn pos`))) "Undefined" "OverrideRootScale" null null))
  (set `self.CurrentSpawnedItem` _returnvalue))

(event `self.ReceiveTick`
  (params (DeltaSeconds :type "Float (single-precision)"))
  (if (`PickupActor.IsBeingCarried` (`self.CurrentSpawnedItem`))
    (bind _returnvalue (`|SpawnActorFromClass` (`self.PickupClass`) (`KismetMathLibrary.Conv_VectorToTransform` (`SceneComponent.K2_GetComponentLocation` (`self.spawn pos`))) "Undefined" "OverrideRootScale" null null))
    (set `self.CurrentSpawnedItem` _returnvalue)))

(fn `UserConstructionScript`)